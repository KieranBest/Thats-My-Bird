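; BP_Lever is a 2D lever that the player toggles with E when standing close to it.
; Tick compares X positions with the player to set OnLever, printing debug text and calling EnableInput in both branches, so input is never disabled.
; When OnLever is true, E flips LeverOn, swaps the crank up/down sprite and adds a new Paper tile map component on each press.
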(event EventBeginPlay)

(event Collision|EventActorBeginOverlap
  (params (OtherActor :type Actor%20Object%20Reference)))

(event EventTick
  (params (DeltaSeconds :type Float%20%28single-precision%29))
  (bind _returnvalue (Game|GetPlayerController 0))
  (Utilities|FlowControl|Sequence
    (:then_0
      (Variables|Default|SetDistance (- (.x (Transformation|GetActorLocation)) (.x (Transformation|GetActorLocation (Game|GetPlayerCharacter 0))))))
    (:then_1
      (Development|PrintString (Utilities|String|ToString(Float) (Variables|Default|GetDistance))))
    (:then_2
      (if (Math|Float|InRange(Float) (Variables|Default|GetDistance) -1e+01 1e+01 false false)
        (Variables|Default|SetOnLever true)
        (Input|EnableInput _returnvalue)
        (Development|PrintString "On")
        (else
          (Variables|Default|SetOnLever false)
          (Input|EnableInput _returnvalue)
          (Development|PrintString "Off"))))))

(event Input|KeyboardEvents|E
  (params (Key :type Key%20Structure :default "None"))
  (:Pressed
    (if (Variables|Default|GetOnLever)
      (AddComponent|AddPaperTileMapComponent false (Class|TileMapBlueprintLibrary|GetTileTransform))
      (if (Variables|Default|GetLeverOn)
        (Variables|Default|SetLeverOn false)
        (Rendering|Components|Sprite|SetSprite (Variables|Default|GetLever) "/Game/Assets/environment/props/crank-up_Sprite.crank-up_Sprite")
        (else
          (Variables|Default|SetLeverOn true)
          (Rendering|Components|Sprite|SetSprite (Variables|Default|GetLever) "/Game/Assets/environment/props/crank-down_Sprite.crank-down_Sprite"))))))

(fn ConstructionScript)